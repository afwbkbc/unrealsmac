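; BP_Planet_Clouds is a randomized, spinning cloud layer for a main menu planet.
; The construction script slightly varies the Clouds component's scale per axis, applies a random root yaw, and randomly flips the cloud material's X and Y through invert parameters on a dynamic instance.
; BeginPlay picks a random spin speed that Tick applies as frame-rate-independent yaw.
; A SetOpacity event drives the material's CloudsOpacity parameter.
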(event Custom|SetOpacity
  (params (Opacity :type Float%20%28single-precision%29))
  (Rendering|Material|SetScalarParameterValue (Variables|Default|GetMaterial) "CloudsOpacity" Opacity :!class /Script/Engine.MaterialInstanceDynamic))

(event EventBeginPlay
  (Variables|Default|SetRotationSpeed (Math|Random|RandomFloatinRange 0.0 0.3)))

(event Collision|EventActorBeginOverlap
  (params (OtherActor :type Actor%20Object%20Reference)))

(event EventTick
  (params (DeltaSeconds :type Float%20%28single-precision%29))
  (Transformation|AddRelativeRotation (Variables|Default|GetClouds) (Math|Rotator|MakeRotator 0.0 0.0 (* (Variables|Default|GetRotationSpeed) DeltaSeconds)) false false))

(fn ConstructionScript
  (bind _returnvalue (Math|Random|RandomFloatinRange 0.0 1.0))
  (bind _clouds (Variables|Default|GetClouds))
  (bind _returnvalue_2 (* _returnvalue 0.5))
  (bind _returnvalue_3 (+ 1e+01 _returnvalue_2))
  (Transformation|SetRelativeScale3D _clouds (Math|Vector|MakeVector _returnvalue_3 _returnvalue_3 _returnvalue_3))
  (bind _returnvalue_4 (Rendering|Material|CreateDynamicMaterialInstance _clouds 0 "/Game/MainMenu/Planet/M_Planet_Clouds.M_Planet_Clouds" "None" :!class /Script/Engine.PrimitiveComponent))
  (bind _output_get (Variables|Default|SetMaterial _returnvalue_4))
  (Utilities|FlowControl|Sequence
    (:then_0
      (Transformation|AddLocalRotation (Variables|Default|GetDefaultSceneRoot) (Math|Rotator|MakeRotator 0.0 0.0 (Math|Random|RandomFloatinRange 0.0 3.6e+02)) false false))
    (:then_1
      (if (Math|Random|RandomBool)
        (Rendering|Material|SetScalarParameterValue _output_get "CloudsInvertX" -1.0 :!class /Script/Engine.MaterialInstanceDynamic)))
    (:then_2
      (if (Math|Random|RandomBool)
        (Rendering|Material|SetScalarParameterValue _output_get "CloudsInvertY" -1.0 :!class /Script/Engine.MaterialInstanceDynamic)))))