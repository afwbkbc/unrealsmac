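; Main menu planet actor that shows a slowly spinning surface wrapped in stacked cloud layers.
; The construction script creates a dynamic surface material driven by FungusDensity and WaterArea.
; BeginPlay randomizes the surface yaw and spawns attached BP_Planet_Clouds layers, while Tick rotates the root.
; SetCloudsDensity turns one density value into clamped per-layer opacities, so layers fade in successively by index.
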(event Custom|SetCloudsDensity
  (params (Density :type Float%20%28single-precision%29))
  (for (_array_element _array_index) (Variables|Default|GetClouds)
    (Default|SetOpacity _array_element (Math|Float|Clamp(Float) (- (* Density (Math|Float|MakeLiteralFloat 1e+01)) (Math|Conversions|ToFloat(Integer) _array_index))))))

(event Custom|SpawnClouds
  (for _index (range 0 (Math|Float|Truncate (Math|Float|MakeLiteralFloat 1e+01)))
    (bind _returnvalue (Game|SpawnActorfromClass "/Game/MainMenu/Planet/BP_Planet_Clouds.BP_Planet_Clouds_C" (Transformation|GetWorldTransform (Variables|Default|GetDefaultSceneRoot)) "Undefined" 0 0))
    (Transformation|AttachActorToActor _returnvalue self "None" "KeepWorld" "KeepRelative" "KeepWorld" true)
    (Utilities|Array|Add (Variables|Default|GetClouds) _returnvalue)))

(event Custom|Rotate
  (params (Delta%20Seconds :type Float%20%28single-precision%29))
  (Transformation|AddRelativeRotation (Variables|Default|GetDefaultSceneRoot) (* (Math|Rotator|MakeRotator 0.0 0.0 0.1) Delta%20Seconds) false false))

(event EventBeginPlay
  (Transformation|AddLocalRotation (Variables|Default|GetPlanetSurface) (Math|Rotator|MakeRotator 0.0 0.0 (Math|Random|RandomFloatinRange 0.0 3.6e+02)) false false)
  (CallFunction|SpawnClouds)
  (CallFunction|SetCloudsDensity 0.5))

(event Collision|EventActorBeginOverlap
  (params (OtherActor :type Actor%20Object%20Reference)))

(event EventTick
  (params (DeltaSeconds :type Float%20%28single-precision%29))
  (CallFunction|Rotate DeltaSeconds))

(fn ConstructionScript
  (bind _returnvalue (Rendering|Material|CreateDynamicMaterialInstance (Variables|Default|GetPlanetSurface) 0 "/Game/MainMenu/Planet/M_Planet_Surface.M_Planet_Surface" "None" :!class /Script/Engine.PrimitiveComponent))
  (Utilities|FlowControl|Sequence
    (:then_0
      (Rendering|Material|SetScalarParameterValue _returnvalue "FungusDensity" (Variables|Default|GetFungusDensity) :!class /Script/Engine.MaterialInstanceDynamic))
    (:then_1
      (Rendering|Material|SetScalarParameterValue _returnvalue "Moisture" (Variables|Default|GetWaterArea) :!class /Script/Engine.MaterialInstanceDynamic))))