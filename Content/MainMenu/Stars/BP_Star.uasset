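; BP_Star is a main-menu star actor that slowly spins a star component and carries a colored light.
; The construction script drives an M_Star dynamic material, component scale and the light from LightColor and Size, with light intensity growing with the square of Size.
; BeginPlay randomizes initial orientation and per-axis spin speeds, which Tick applies as frame-rate-independent local rotation.
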(event Custom|InitRotation
  (bind _returnvalue (Math|Float|MakeLiteralFloat 1e+01))
  ;[1 1 1] Add random initial rotation
  (Transformation|AddLocalRotation (Variables|Default|GetStar) (Math|Rotator|MakeRotator (Math|Random|RandomFloatinRange 0.0 3.6e+02) (Math|Random|RandomFloatinRange 0.0 3.6e+02) (Math|Random|RandomFloatinRange 0.0 3.6e+02)) false false)
  ;[1 1 1] Randomize rotation speed
  (Variables|Default|SetRotationX (Math|Random|RandomFloatinRange (stale _result) _returnvalue))
  (Variables|Default|SetRotationY (Math|Random|RandomFloatinRange (stale _result) _returnvalue))
  (Variables|Default|SetRotationZ (Math|Random|RandomFloatinRange (stale _result) _returnvalue)))

(event Custom|Rotate
  (params (Delta%20Seconds :type Float%20%28single-precision%29))
  (Transformation|AddLocalRotation (Variables|Default|GetStar) (Math|Rotator|MakeRotator (* (Variables|Default|GetRotationX) Delta%20Seconds) (* (Variables|Default|GetRotationY) Delta%20Seconds) (* (Variables|Default|GetRotationZ) Delta%20Seconds)) false false))

(event EventBeginPlay
  (CallFunction|InitRotation))

(event Collision|EventActorBeginOverlap
  (params (OtherActor :type Actor%20Object%20Reference)))

(event EventTick
  (params (DeltaSeconds :type Float%20%28single-precision%29))
  (CallFunction|Rotate DeltaSeconds))

(fn ConstructionScript
  (bind _size (Variables|Default|GetSize))
  (bind _lightcolor (Variables|Default|GetLightColor))
  (bind (_b _g _r) (Math|Color|BreakColor _lightcolor))
  ;[1 1 1] Update star color and intensity
  (bind _returnvalue (Rendering|Material|CreateDynamicMaterialInstance "/Game/MainMenu/Stars/M_Star.M_Star" "None" :!class /Script/Engine.KismetMaterialLibrary))
  (bind _output_get (Variables|Default|SetMaterial _returnvalue))
  (Utilities|FlowControl|Sequence
    (:then_0
      (Rendering|Material|SetMaterial (Variables|Default|GetStar) 0 _output_get))
    (:then_1
      (Rendering|Material|SetScalarParameterValue _output_get "LightColorR" (/ (Math|Conversions|ToFloat(Byte) _r) 256.0) :!class /Script/Engine.MaterialInstanceDynamic))
    (:then_2
      (Rendering|Material|SetScalarParameterValue _output_get "LightColorG" (/ (Math|Conversions|ToFloat(Byte) _g) 256.0) :!class /Script/Engine.MaterialInstanceDynamic))
    (:then_3
      (Rendering|Material|SetScalarParameterValue _output_get "LightColorB" (/ (Math|Conversions|ToFloat(Byte) _b) 256.0) :!class /Script/Engine.MaterialInstanceDynamic))
    (:then_4
      (Rendering|Material|SetScalarParameterValue _output_get "LightIntensity" (Variables|Default|GetSize) :!class /Script/Engine.MaterialInstanceDynamic))
    (:then_5
      ;[1 1 1] Update scale and size
      (Class|PointLightComponent|SetSourceRadius (Variables|Default|GetLight) _size)
      (Transformation|SetRelativeScale3D (Variables|Default|GetStar) (Math|Vector|MakeVector _size _size _size))
      (Rendering|Components|Light|SetIntensity (Variables|Default|GetLight) (* 2e+05 (Math|Float|Square _size)))
      (Rendering|Components|Light|SetLightColor (Variables|Default|GetLight) (Math|Conversions|ToLinearColor(Color) (Variables|Default|GetLightColor)) true))))