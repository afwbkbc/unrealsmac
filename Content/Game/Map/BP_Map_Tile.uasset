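; BP_Map_Tile is a map tile actor that builds its own procedural mesh from predefined vertices, triangles and UVs.
; Init applies per-corner elevations scaled by 100 to the outer vertices and sets the center vertex to their six-way average height.
; It then creates the mesh section, applies M_Map_Tile and reveals the mesh, which the construction script hides.
; Init's XPos and YPos inputs are unused.
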(event Custom|Init
  (params (XPos :type Integer) (YPos :type Integer) (Elevation :type Array%20of%20Floats%20%28single-precision%29))
  (bind _mesh (Variables|Default|GetMesh))
  (CallFunction|UpdateVertices Elevation)
  (Class|ProceduralMeshComponent|CreateMeshSectionLinearColor _mesh 0 (Variables|Default|GetVertices) (Variables|Default|GetTriangles) 0 (Variables|Default|GetUV0) 0 0 0 0 0 false)
  (Rendering|Material|SetMaterial _mesh 0 "/Game/Game/Map/M_Map_Tile.M_Map_Tile")
  (Rendering|SetVisibility _mesh true false))

(event Custom|UpdateVertices
  (params (Elevation :type Array%20of%20Floats%20%28single-precision%29))
  (bind _vertices (Variables|Default|GetVertices))
  (bind _vertices_2 (Variables|Default|GetVertices))
  (bind _output (Utilities|Array|Get(acopy) _vertices_2))
  (bind (_x _y) (Math|Vector|BreakVector _output))
  (Variables|Default|SetElevation 0.0)
  (for (_array_element _array_index) Elevation
    (Utilities|Array|SetArrayElem _vertices (+ _array_index 1) (Math|Vector|MakeVector (.X (Math|Vector|BreakVector (Utilities|Array|Get(acopy) _vertices (+ _array_index 1)))) (.Y (Math|Vector|BreakVector (Utilities|Array|Get(acopy) _vertices (+ _array_index 1)))) (* _array_element 1e+02)))
    (Variables|Default|SetElevation (+ (Variables|Default|GetElevation) (* _array_element 1e+02))))
  (bind _output_get (Variables|Default|SetElevation (/ (Variables|Default|GetElevation) 6.0)))
  (Utilities|Array|SetArrayElem _vertices_2 0 (Math|Vector|MakeVector _x _y _output_get)))

(event EventBeginPlay)

(event Collision|EventActorBeginOverlap
  (params (OtherActor :type Actor%20Object%20Reference)))

(event EventTick
  (params (DeltaSeconds :type Float%20%28single-precision%29)))

(fn ConstructionScript
  (Rendering|SetVisibility (Variables|Default|GetMesh) false false))