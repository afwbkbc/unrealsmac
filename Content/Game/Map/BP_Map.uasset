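; BP_Map generates a planet's map as a centred, square grid of hex tiles sized from PlanetInfo.PlanetSize and PlanetScale.
; Generate spawns BP_Map_Tile actors with staggered offsets on alternating indices and stores them in a flattened Tiles array.
; Each tile's Init receives six vertex elevations, each averaging two 1D Perlin samples of world X and Y, shifted by random seeds from BeginPlay.
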(event Custom|Generate
  (params (PlanetInfo :type T%20Planet%20Info%20Structure))
  (bind _planetscale (Variables|Default|GetPlanetScale))
  (bind _perlinscale (Variables|Default|GetPerlinScale))
  (bind _planetscale_2 (Variables|Default|GetPlanetScale))
  (bind _elevation (Variables|Default|GetElevation))
  (bind _tilescale (Variables|Default|GetTileScale))
  (bind _returnvalue (/ _perlinscale _planetscale_2))
  (bind _returnvalue_2 (* _planetscale (.planetsize PlanetInfo)))
  (bind _returnvalue_3 (Math|Float|Floor _returnvalue_2))
  (bind _returnvalue_4 (/ _returnvalue_2 2.0))
  (Utilities|FlowControl|Sequence
    (:then_0
      (bind _output_get (Variables|Default|SetMaxX _returnvalue_3))
      (Variables|Default|SetMaxY _output_get))
    (:then_1
      (for _index (range 0 (Variables|Default|GetMaxX))
        (for _index_2 (range 0 (Variables|Default|GetMaxY))
          ;[1 1 1] Tile creation
          (bind _returnvalue_5 (Game|SpawnActorfromClass "/Game/Game/Map/BP_Map_Tile.BP_Map_Tile_C" (Math|Transform|MakeTransform (Math|Vector|MakeVector (* (- (* (Math|Conversions|ToFloat(Integer) _index) 0.5) (* _returnvalue_4 0.5)) _tilescale) (* (- (* (- (+ (Math|Conversions|ToFloat(Integer) _index_2) (* (Math|Integer|%(Integer) _index 2) -0.125)) (* (- 1 (Math|Integer|%(Integer) _index 2)) 0.625)) 1.5) (* _returnvalue_4 1.5)) _tilescale) 0.0)) "Undefined" 0 0))
          (Utilities|Array|Insert (Variables|Default|GetTiles) _returnvalue_5 (+ (* _index _returnvalue_3) _index_2))
          ;[1 1 1] Generate heightmap
          (Utilities|Array|Clear _elevation)
          (for _index_3 (range 0 5)
            (Utilities|Array|Add _elevation (/ (+ (Class|KismetMathLibrary|PerlinNoise1D (* (+ (+ (* (- (* (Math|Conversions|ToFloat(Integer) _index) 0.5) (* _returnvalue_4 0.5)) _tilescale) (Math|Conversions|ToFloat(Integer) (Variables|Default|GetSeedX))) (.X (Math|Vector2D|BreakVector2D (* (Utilities|Array|Get(acopy) (Variables|Default|GetTileVertexOffset) _index_3) (Variables|Default|GetTileScale))))) _returnvalue)) (Class|KismetMathLibrary|PerlinNoise1D (* (+ (+ (* (- (* (- (+ (Math|Conversions|ToFloat(Integer) _index_2) (* (Math|Integer|%(Integer) _index 2) -0.125)) (* (- 1 (Math|Integer|%(Integer) _index 2)) 0.625)) 1.5) (* _returnvalue_4 1.5)) _tilescale) (Math|Conversions|ToFloat(Integer) (Variables|Default|GetSeedY))) (.Y (Math|Vector2D|BreakVector2D (* (Utilities|Array|Get(acopy) (Variables|Default|GetTileVertexOffset) _index_3) (Variables|Default|GetTileScale))))) _returnvalue))) 2.0)))
          ;[1 1 1] Initialize Tile
          (Default|Init _returnvalue_5 _index _index_2 _elevation))))))

(event EventBeginPlay
  (bind _returnvalue (Math|Random|RandomIntegerinRange 0 9999))
  (Variables|Default|SetSeedX _returnvalue)
  (Variables|Default|SetSeedY _returnvalue))

(event Collision|EventActorBeginOverlap
  (params (OtherActor :type Actor%20Object%20Reference)))

(event EventTick
  (params (DeltaSeconds :type Float%20%28single-precision%29)))

(fn ConstructionScript)